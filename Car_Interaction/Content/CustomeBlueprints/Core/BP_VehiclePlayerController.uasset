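; BP_VehiclePlayerController manages Health, OxygenLevel and WaterLevel survival stats and sprint speed for BP_ThirdPersonCharacter.
; Left Shift toggles retriggerable-delay loops that set walk speed and drain stats, with sprinting cancelled at low oxygen or water and low oxygen costing health.
; Tick drains standing oxygen via a Delay and runs DoOnce-gated depletion checks that start looping damage timers.
; Oxygen regeneration and the car-entry montage are unwired.
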(event Custom|UseOxygen
  (Variables|CharacterAttributes|SetOxygenLevel (- (Variables|CharacterAttributes|GetOxygenLevel) 2.0))
  (if (<= (Variables|CharacterAttributes|GetOxygenLevel) 5.0)
    (Variables|Default|SetIsRunning? false)
    (bind _asbp_third_person_character (Utilities|Casting|CastToBP_ThirdPersonCharacter (Game|GetPlayerCharacter 0)))
    (Variables|/Script/Engine.CharacterMovementComponent|SetMaxWalkSpeed (Variables|/Script/Engine.Character|GetCharacterMovement _asbp_third_person_character) 3e+02)
    (else
      (Development|PrintString (Utilities|String|ToString(Float) (Variables|CharacterAttributes|GetOxygenLevel))))))

(event Custom|CheckOxygenLevel
  (Utilities|FlowControl|DoOnce false
    (:Completed
      (if (<= (Variables|CharacterAttributes|GetOxygenLevel) 0.0)
        (Utilities|Time|SetTimerbyEvent (delegate Custom|DecreaseHealthOxgenLevel) (Variables|Default|GetOxygenTimer) true)))))

(event Custom|DecreseHealthWaterLevel
  (Utilities|FlowControl|RetriggerableDelay 0.2)
  (Variables|CharacterAttributes|SetHealth (- (Variables|CharacterAttributes|GetHealth) 1.0))
  (Variables|Default|SetWaterLevelTimer 0.0))

(event Custom|CheckWaterLevel
  (Utilities|FlowControl|DoOnce false
    (:Completed
      (if (<= (Variables|CharacterAttributes|GetWaterLevel) 0.0)
        (Utilities|Time|SetTimerbyEvent (delegate Custom|DecreseHealthWaterLevel) (Variables|Default|GetWaterLevelTimer) true)))))

(event Custom|DecreaseHealthOxgenLevel
  (Development|PrintString "Hello")
  (Utilities|FlowControl|RetriggerableDelay 0.2)
  (Variables|CharacterAttributes|SetHealth (- (Variables|CharacterAttributes|GetHealth) 2.0))
  (Variables|Default|SetOxygenTimer 0.0))

(event Custom|UseOxygen_If_Standing
  (if (not (Variables|Default|GetIsRunning?))
    (Variables|CharacterAttributes|SetOxygenLevel (- (Variables|CharacterAttributes|GetOxygenLevel) 1.0))))

(event Custom|DecreaseHealth
  (if (<= (Variables|CharacterAttributes|GetOxygenLevel) 5.0) :!label _label
    (Utilities|FlowControl|RetriggerableDelay 0.2)
    (Variables|CharacterAttributes|SetHealth (- (Variables|CharacterAttributes|GetHealth) 1.0))
    (if (not (<= (Variables|CharacterAttributes|GetHealth) 0.0))
      (goto _label))))

(event Custom|UseWater
  (Variables|CharacterAttributes|SetWaterLevel (- (Variables|CharacterAttributes|GetWaterLevel) 1.0))
  (if (<= (Variables|CharacterAttributes|GetWaterLevel) 5.0)
    (Variables|Default|SetIsRunning? false)
    (bind _asbp_third_person_character (Utilities|Casting|CastToBP_ThirdPersonCharacter (Game|GetPlayerCharacter 0)))
    (Variables|/Script/Engine.CharacterMovementComponent|SetMaxWalkSpeed (Variables|/Script/Engine.Character|GetCharacterMovement _asbp_third_person_character) 3e+02)
    (else
      (Development|PrintString (Utilities|String|ToString(Float) (Variables|CharacterAttributes|GetWaterLevel))))))

(event Custom|Increase_Oxygen
  (Variables|CharacterAttributes|SetOxygenLevel (+ (Variables|CharacterAttributes|GetOxygenLevel) 2.0))
  (if (>= (Variables|CharacterAttributes|GetOxygenLevel) 1e+02)
    (Variables|Default|SetCanIncreaseStamina? false)
    (else
      (Variables|Default|SetCanIncreaseStamina? true))))

(event EventTick
  (params (DeltaSeconds :type Float%20%28single-precision%29))
  (CallFunction|CheckOxygenLevel)
  (CallFunction|CheckWaterLevel)
  (Utilities|FlowControl|Delay 2.0)
  (CallFunction|UseOxygenifStanding))

(event Input|KeyboardEvents|LeftShift
  (params (Key :type Key%20Structure :default "None"))
  (:Pressed
    (Variables|Default|SetIsRunning? true)
    (bind _asbp_third_person_character (Utilities|Casting|CastToBP_ThirdPersonCharacter (Game|GetPlayerCharacter 0)))
    (Utilities|IsValid _asbp_third_person_character
      (:Is%20Valid
        (Variables|/Script/Engine.CharacterMovementComponent|SetMaxWalkSpeed (Variables|/Script/Engine.Character|GetCharacterMovement _asbp_third_person_character) 6e+02 :!label _label)
        (Utilities|FlowControl|RetriggerableDelay 0.2)
        (CallFunction|UseOxygen)
        (CallFunction|UseWater)
        (CallFunction|DecreaseHealth)
        (if (Variables|Default|GetIsRunning?)
          (goto _label)))))
  (:Released
    (Variables|Default|SetIsRunning? false)
    (bind _asbp_third_person_character_2 (Utilities|Casting|CastToBP_ThirdPersonCharacter (Game|GetPlayerCharacter 0)))
    (Utilities|IsValid _asbp_third_person_character_2
      (:Is%20Valid
        (Variables|/Script/Engine.CharacterMovementComponent|SetMaxWalkSpeed (Variables|/Script/Engine.Character|GetCharacterMovement _asbp_third_person_character_2) 3.5e+02 :!label _label_2)
        (Utilities|FlowControl|RetriggerableDelay 0.2)
        (CallFunction|UseOxygenifStanding)
        (CallFunction|DecreaseHealth)
        (if (not (Variables|Default|GetIsRunning?))
          (goto _label_2))))))

(fn ConstructionScript)